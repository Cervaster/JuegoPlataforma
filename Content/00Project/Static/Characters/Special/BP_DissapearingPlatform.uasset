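; BP_DissapearingPlatform is a platform that periodically vanishes and returns.
; After an initial delay, a looping timer fires ShowOrHide, which toggles the Cube's collision and the actor's visibility.
; When Shown is false, the construction script hides the actor and the toggle never reveals it, so only collision cycles on an invisible platform.
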(event Custom|ShowOrHide
  (bind _cube (Variables|Default|GetCube))
  (if (Variables|Default|GetIsHidden)
    (if (Variables|Default|GetShown)
      (Rendering|SetActorHiddenInGame false))
    (Collision|SetCollisionEnabled _cube "QueryAndPhysics")
    (Variables|Default|SetIsHidden false)
    (else
      (Rendering|SetActorHiddenInGame true)
      (Collision|SetCollisionEnabled _cube "NoCollision")
      (Variables|Default|SetIsHidden true))))

(event EventBeginPlay
  (Utilities|FlowControl|Delay (Variables|Default|GetDelay))
  (Utilities|Time|SetTimerbyEvent (delegate Custom|ShowOrHide) (Variables|Default|GetTime) true))

(fn ConstructionScript
  (if (not (Variables|Default|GetShown))
    (Rendering|SetActorHiddenInGame true)))